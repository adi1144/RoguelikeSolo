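; ProjectileCannonBP is a cannon actor that fires a magic projectile on a fixed interval.
; A looping timer started on BeginPlay spawns MagicProjectileBP at the actor's own location and rotation.
; Tick turns the Arrow component toward player 0's pawn by setting a look-at rotation as its relative rotation.
; The spawn transform ignores the Arrow, so that aim does not steer the projectiles.
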(event Custom|OnTimeElapsed
  (Game|SpawnActorfromClass "/Game/RogueLike/MagicProjectileBP.MagicProjectileBP_C" (Math|Transform|MakeTransform (Transformation|GetActorLocation) (Transformation|GetActorRotation)) "Undefined" 0 0))

(event EventBeginPlay
  (Utilities|Time|SetTimerbyEvent (delegate Custom|OnTimeElapsed) 2.0 true))

(event EventTick
  (params (DeltaSeconds :type Float%20%28single-precision%29))
  (Transformation|SetRelativeRotation (Variables|Default|GetArrow) (Math|Rotator|FindLookatRotation (Transformation|GetActorLocation) (Transformation|GetActorLocation (Game|Player|GetPlayerPawn 0))) false false))

(fn ConstructionScript)